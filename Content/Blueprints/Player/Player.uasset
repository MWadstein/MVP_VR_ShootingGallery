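; Player Blueprint for a motion-controller shooter that fires a hitscan gun and tracks the player's score.
; Either trigger runs a line trace from the gun's muzzle point, spawns an impact particle, and notifies hit enemies or in-game menus through Blueprint interfaces.
; Score add and reset events update a score display actor, found at BeginPlay by its interface.
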(event EventAddtoScore
  (params (Value :type Integer))
  (bind _output_get (Variables|Default|SetPlayerScore (+ (Variables|Default|GetPlayerScore) Value)))
  (Class|BPIinGamePlayerScoreBP|UpdateDisplayedScore(Message) (Variables|Default|GetScoreBP) _output_get))

(event EventResetScore
  (bind _output_get (Variables|Default|SetPlayerScore 0))
  (Class|BPIinGamePlayerScoreBP|UpdateDisplayedScore(Message) (Variables|Default|GetScoreBP) _output_get))

(event EventBeginPlay
  (bind _outactors (Actor|GetAllActorswithInterface "/Game/Blueprints/Interfaces/BPI_InGamePlayerScoreBP.BPI_InGamePlayerScoreBP_C"))
  (Variables|Default|SetScoreBP (Utilities|Array|Get(acopy) _outactors)))

(event Input|KeyboardEvents|MotionControllerLeftTrigger
  (params (Key :type Key%20Structure :default "AnyKey"))
  (bind _gunfiringstartpoint (Variables|Default|GetGunFiringStartPoint))
  (bind _returnvalue (Transformation|GetWorldLocation _gunfiringstartpoint))
  (:Pressed
    (bind (_outhit _returnvalue_2) (Collision|LineTraceByChannel _returnvalue (+ _returnvalue (* (Math|Vector|GetForwardVector (Transformation|GetWorldRotation _gunfiringstartpoint)) 1.5e+03)) "TraceTypeQuery1" false 0 "None"))
    (if _returnvalue_2
      (Variables|Default|SetHitActor (.HitActor (Collision|BreakHitResult _outhit)))
      (Effects|SpawnEmitteratLocation "/Game/Particles/HitParticle.HitParticle" (.ImpactPoint (Collision|BreakHitResult _outhit)) (Math|Rotator|MakeRotfromZ (.ImpactNormal (Collision|BreakHitResult _outhit))))
      (if (Utilities|DoesObjectImplementInterface (Variables|Default|GetHitActor) "/Game/Blueprints/Interfaces/BPI_Enemy.BPI_Enemy_C")
        (Class|BPIEnemy|WasHit(Message) (Variables|Default|GetHitActor))
        (elif (Utilities|DoesObjectImplementInterface (Variables|Default|GetHitActor) "/Game/Blueprints/Interfaces/BPI_InGameMenuBP.BPI_InGameMenuBP_C")
          (Class|BPIinGameMenuBP|InteractwithMenu(Message) (Variables|Default|GetHitActor) (.HitComponent (Collision|BreakHitResult _outhit))))))))

(event Input|KeyboardEvents|MotionControllerRightTrigger
  (params (Key :type Key%20Structure :default "AnyKey"))
  (bind _gunfiringstartpoint (Variables|Default|GetGunFiringStartPoint))
  (bind _returnvalue (Transformation|GetWorldLocation _gunfiringstartpoint))
  (:Pressed
    (bind (_outhit _returnvalue_2) (Collision|LineTraceByChannel _returnvalue (+ _returnvalue (* (Math|Vector|GetForwardVector (Transformation|GetWorldRotation _gunfiringstartpoint)) 1.5e+03)) "TraceTypeQuery1" false 0 "None"))
    (if _returnvalue_2
      (Variables|Default|SetHitActor (.HitActor (Collision|BreakHitResult _outhit)))
      (Effects|SpawnEmitteratLocation "/Game/Particles/HitParticle.HitParticle" (.ImpactPoint (Collision|BreakHitResult _outhit)) (Math|Rotator|MakeRotfromZ (.ImpactNormal (Collision|BreakHitResult _outhit))))
      (if (Utilities|DoesObjectImplementInterface (Variables|Default|GetHitActor) "/Game/Blueprints/Interfaces/BPI_Enemy.BPI_Enemy_C")
        (Class|BPIEnemy|WasHit(Message) (Variables|Default|GetHitActor))
        (elif (Utilities|DoesObjectImplementInterface (Variables|Default|GetHitActor) "/Game/Blueprints/Interfaces/BPI_InGameMenuBP.BPI_InGameMenuBP_C")
          (Class|BPIinGameMenuBP|InteractwithMenu(Message) (Variables|Default|GetHitActor) (.HitComponent (Collision|BreakHitResult _outhit))))))))

(fn ConstructionScript)